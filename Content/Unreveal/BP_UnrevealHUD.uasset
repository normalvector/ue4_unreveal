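; HUD Blueprint that shows the WBP_Unreveal widget and draws a transparent BLUI (BluEye) browser across the whole screen.
; SetupBLUI creates and initializes the browser with a local UI page as its default URL.
; BeginPlay issues a Google LoadURL before that setup runs, so BluEye is not yet created by this Blueprint at that point.
; Each DrawHUD pumps the BLUI event loop, resizes the browser when screen size changes, and draws its texture.
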(event `self.ReceiveBeginPlay`
  (`|ExecutionSequence`
    (:`then_0`
      (bind _returnvalue (`|CreateWidget` "/Game/Unreveal/WBP_Unreveal.WBP_Unreveal_C"))
      (`UserWidget.AddToViewport` _returnvalue 0)
      (`BluEye.LoadURL` (`self.BluEye`) "http://google.com"))
    (:`then_1`
      (`self.SetupBLUI`))))

(event `self.ReceiveDrawHUD`
  (params (SizeX :type Integer) (SizeY :type Integer))
  (`|ExecutionSequence`
    (:`then_0`
      (`BluBlueprintFunctionLibrary.RunBluEventLoop`))
    (:`then_1`
      (`self.HandleResize` SizeX SizeY))
    (:`then_2`
      (`self.DrawTexture` (`BluEye.GetTexture` (`self.BluEye`)) 0.0 0.0 (`KismetMathLibrary.Conv_IntToDouble` SizeX) (`KismetMathLibrary.Conv_IntToDouble` SizeY) 0.0 0.0 1.0 1.0))))

(fn `HandleResize`
  (params (SizeX :type Integer) (SizeY :type Integer))
  (if (or (!= SizeX (`BluEye.Width` (`self.BluEye`))) (!= SizeY (`BluEye.Height` (`self.BluEye`))))
    (`BluEye.ResizeBrowser` (`self.BluEye`) SizeX SizeY)))

(fn `SetupBLUI`
  (bind _blueye (`self.BluEye`))
  (`|ExecutionSequence`
    (:`then_0`
      ;[1 1 1] Create BluEye
      (set `self.BluEye` (`BluBlueprintFunctionLibrary.NewBluEye`)))
    (:`then_1`
      ;[1 1 1] Configure BluEye
      (set `BluEye.DefaultURL` "blui://UI/index.html" _blueye)
      (set `BluEye.bIsTransparent` true _blueye)
      (set `BluEye.bEnabled` true _blueye))
    (:`then_2`
      ;[1 1 1] Start the BluEye
      (`BluEye.init` (`self.BluEye`)))))

(fn `UserConstructionScript`)